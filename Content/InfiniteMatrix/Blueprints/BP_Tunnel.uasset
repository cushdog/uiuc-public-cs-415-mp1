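; BP_Tunnel is an endless-tunnel segment with a rotating holed wall; RandomizeWall picks its mesh and roll.
; The player's overlap with TriggerZone requests another segment from TunnelSpawner, destroys this one and adds score, while projectiles entering it are destroyed.
; Wall hits cost the player health and score and remove the wall, or trigger death on last health.
; The player's Capsule overlap spawns one randomly placed enemy and one healthpack offset from it.
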(event OnComponentBeginOverlap(TriggerZone)
  (params (OverlappedComponent :type Primitive%20Component%20Object%20Reference) (OtherActor :type Actor%20Object%20Reference) (OtherComp :type Primitive%20Component%20Object%20Reference) (OtherBodyIndex :type Integer) (bFromSweep :type Boolean) (SweepResult :type Hit%20Result%20Structure%20%28by%20ref%29))
  ;[1 1 1] Spawn More Tunnels/Destroy Previous Tunnel
  (Utilities|Casting|CastToBP_Player OtherActor
    (:then
      (Default|SpawnTunnelatSpawnPoint (Variables|Default|GetTunnelSpawner))
      (Actor|DestroyActor)
      ;[1 1 1] Update Score
      (bind _asbp_player (Utilities|Casting|CastToBP_Player OtherActor))
      (Math|Float|IncrementFloat (Variables|/Game/InfiniteMatrix/Blueprints/BP_Player.BP_Player_C|GetScore _asbp_player)
        (:%20%20
          (Default|UpdateCounterText (Variables|/Game/InfiniteMatrix/Blueprints/BP_Player.BP_Player_C|GetHealthHUD _asbp_player)))))
    (:CastFailed
      ;[1 1 1] Destroy Projectile if Collides with Tunnel Wall
      (bind _asbp_projectile (Utilities|Casting|CastToBP_Projectile OtherActor))
      (Actor|DestroyActor _asbp_projectile))))

(event OnComponentHit(WallMesh)
  (params (HitComponent :type Primitive%20Component%20Object%20Reference) (OtherActor :type Actor%20Object%20Reference) (OtherComp :type Primitive%20Component%20Object%20Reference) (NormalImpulse :type Vector :default "0, 0, 0") (Hit :type Hit%20Result%20Structure%20%28by%20ref%29))
  ;[1 1 1] General Health Deccrement Function
  (bind _asbp_player (Utilities|Casting|CastToBP_Player OtherActor))
  (if (<= (Variables|/Game/InfiniteMatrix/Blueprints/BP_Player.BP_Player_C|GetHealth _asbp_player) (Math|Float|MakeLiteralFloat 1.0))
    (Variables|/Game/InfiniteMatrix/Blueprints/BP_Player.BP_Player_C|SetIsDead _asbp_player true)
    (Default|DisplayRestart _asbp_player)
    (else
      (bind _result (Math|Float|DecrementFloat (Variables|/Game/InfiniteMatrix/Blueprints/BP_Player.BP_Player_C|GetHealth _asbp_player))
        (:%20%20
          (Variables|/Game/InfiniteMatrix/Blueprints/BP_Player.BP_Player_C|SetHealth _asbp_player _result)
          (bind _result_2 (Math|Float|DecrementFloat (Variables|/Game/InfiniteMatrix/Blueprints/BP_Player.BP_Player_C|GetScore _asbp_player))
            (:%20%20
              (Variables|/Game/InfiniteMatrix/Blueprints/BP_Player.BP_Player_C|SetScore _asbp_player _result_2)
              (if (> (Variables|/Game/InfiniteMatrix/Blueprints/BP_Player.BP_Player_C|GetScore _asbp_player) 0.0)
                (Default|UpdateCounterText (Variables|/Game/InfiniteMatrix/Blueprints/BP_Player.BP_Player_C|GetHealthHUD _asbp_player)))
              (Default|UpdateHealthText (Variables|/Game/InfiniteMatrix/Blueprints/BP_Player.BP_Player_C|GetHealthHUD _asbp_player))
              (Components|DestroyComponent (Variables|Default|GetWallMesh)))))))))

(event OnComponentBeginOverlap(Capsule)
  (params (OverlappedComponent :type Primitive%20Component%20Object%20Reference) (OtherActor :type Actor%20Object%20Reference) (OtherComp :type Primitive%20Component%20Object%20Reference) (OtherBodyIndex :type Integer) (bFromSweep :type Boolean) (SweepResult :type Hit%20Result%20Structure%20%28by%20ref%29))
  (bind _spawntrigger (Variables|Default|GetSpawnTrigger))
  (bind _spawntrigger_2 (Variables|Default|GetSpawnTrigger))
  (bind _returnvalue (Transformation|GetWorldLocation _spawntrigger))
  (bind _boxextent (Variables|/Script/Engine.BoxComponent|GetBoxExtent _spawntrigger))
  (bind _returnvalue_2 (Math|Random|RandomPointinBoundingBox _returnvalue _boxextent))
  (Utilities|Casting|CastToBP_Player OtherActor)
  ;[1 1 1] Spawn an Enemy Randomly
  (if (< (Variables|Default|GetNumEnemySpawned) 1)
    (bind _returnvalue_3 (Game|SpawnActorfromClass "/Game/InfiniteMatrix/Blueprints/BP_Enemy.BP_Enemy_C" (Math|Conversions|ToTransform(Vector) (Math|Random|RandomPointinBoundingBox (Transformation|GetWorldLocation _spawntrigger_2) (Variables|/Script/Engine.BoxComponent|GetBoxExtent _spawntrigger_2))) "Undefined" "MultiplyWithRoot" 0 0))
    (bind _result (Math|Integer|IncrementInt (Variables|Default|GetNumEnemySpawned))
      (:%20%20
        (Variables|Default|SetNumEnemySpawned _result)
        (bind _output_get (Variables|Default|SetSpawnXEnemy (.x (Transformation|GetWorldLocation (Variables|/Game/InfiniteMatrix/Blueprints/BP_Enemy.BP_Enemy_C|GetSphere _returnvalue_3)))))
        (Development|PrintString (Utilities|String|ToString(Float) _output_get)))))
  (if (< (Variables|Default|GetNumberofHealthSpawned) 1)
    ;[1 1 1] Spawn Healthpack Randomly
    (Game|SpawnActorfromClass "/Game/InfiniteMatrix/Blueprints/BP_Healthpack.BP_Healthpack_C" (Math|Transform|MakeTransform (Math|Vector|MakeVector (- (Variables|Default|GetSpawnXEnemy) (Math|Random|RandomFloatinRange 1e+02 2e+02)) (.y _returnvalue_2) (+ (.z _returnvalue_2) (Math|Random|RandomFloatinRange -1e+02 1e+02))) "0, 0, 0" "1.000000,1.000000,1.000000") "Undefined" "MultiplyWithRoot" 0 0)
    (bind _result_2 (Math|Integer|IncrementInt (Variables|Default|GetNumberofHealthSpawned))
      (:%20%20
        (Variables|Default|SetNumberofHealthSpawned _result_2)))))

(event EventBeginPlay)

(event EventTick
  (params (DeltaSeconds :type Float%20%28single-precision%29))
  (bind _wallmesh (Variables|Default|GetWallMesh))
  ;[1 1 1] Add Rotation to Tunnel Walls
  (if (Utilities|IsValid _wallmesh)
    (Transformation|AddLocalRotation _wallmesh (Math|Rotator|MakeRotator (* DeltaSeconds (Variables|Default|GetRotateSpeed)) 0.0 0.0) false false)))

(fn ConstructionScript)

(fn RandomizeWall
  (Components|StaticMesh|SetStaticMesh (Variables|Default|GetWallMesh) (Utilities|Select :Index (Math|Random|RandomIntegerinRange 0 3) :Option%200 "/Game/InfiniteMatrix/Meshes/SM_Hole_01.SM_Hole_01" :Option%201 "/Game/InfiniteMatrix/Meshes/SM_Hole_02.SM_Hole_02" :Option%202 "/Game/InfiniteMatrix/Meshes/SM_Hole_03.SM_Hole_03" :Option%203 "/Game/InfiniteMatrix/Meshes/SM_Hole_04.SM_Hole_04"))
  (Transformation|AddLocalRotation (Variables|Default|GetWallMesh) (Math|Rotator|MakeRotator (Math|Random|RandomFloatinRange 0.0 3.6e+02) 0.0 0.0) false false))