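; BP_Enemy is an enemy actor that damages the player on collision and awards score when a projectile destroys it.
; A Rocket_ball hit on BP_Player either lowers health and updates the HUD or, at last health, flags death and shows restart, then destroys the enemy.
; A Sphere overlap with BP_Projectile destroys the enemy and increments score through the projectile's player reference.
; A timer started at BeginPlay removes it after a fixed lifetime.
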(event OnComponentHit(rocket_ball)
  (params (HitComponent :type Primitive%20Component%20Object%20Reference) (OtherActor :type Actor%20Object%20Reference) (OtherComp :type Primitive%20Component%20Object%20Reference) (NormalImpulse :type Vector :default "0, 0, 0") (Hit :type Hit%20Result%20Structure%20%28by%20ref%29))
  (bind _asbp_player (Utilities|Casting|CastToBP_Player OtherActor))
  ;[1 1 1] Handle Collision with Player
  (if (<= (Variables|/Game/InfiniteMatrix/Blueprints/BP_Player.BP_Player_C|GetHealth _asbp_player) (Math|Float|MakeLiteralFloat 1.0))
    (Variables|/Game/InfiniteMatrix/Blueprints/BP_Player.BP_Player_C|SetIsDead _asbp_player true)
    (Default|DisplayRestart _asbp_player)
    (else
      (Math|Float|DecrementFloat (Variables|/Game/InfiniteMatrix/Blueprints/BP_Player.BP_Player_C|GetHealth _asbp_player)
        (:%20%20
          (Default|UpdateHealthText (Variables|/Game/InfiniteMatrix/Blueprints/BP_Player.BP_Player_C|GetHealthHUD _asbp_player))))))
  (Actor|DestroyActor))

(event OnComponentBeginOverlap(Sphere)
  (params (OverlappedComponent :type Primitive%20Component%20Object%20Reference) (OtherActor :type Actor%20Object%20Reference) (OtherComp :type Primitive%20Component%20Object%20Reference) (OtherBodyIndex :type Integer) (bFromSweep :type Boolean) (SweepResult :type Hit%20Result%20Structure%20%28by%20ref%29))
  ;[1 1 1] Handle Score Increment
  (bind _asbp_projectile (Utilities|Casting|CastToBP_Projectile OtherActor))
  (Actor|DestroyActor)
  (Math|Float|IncrementFloat (Variables|/Game/InfiniteMatrix/Blueprints/BP_Player.BP_Player_C|GetScore (Variables|/Game/InfiniteMatrix/Blueprints/BP_Projectile.BP_Projectile_C|GetForwardSpeedPlayer _asbp_projectile))
    (:%20%20
      (Default|UpdateCounterText (Variables|/Game/InfiniteMatrix/Blueprints/BP_Player.BP_Player_C|GetHealthHUD (Variables|/Game/InfiniteMatrix/Blueprints/BP_Projectile.BP_Projectile_C|GetForwardSpeedPlayer _asbp_projectile))))))

(event Custom|DestroySelf
  ;[1 1 1] Destroy Self when Player Passes
  (Actor|DestroyActor))

(event EventBeginPlay
  ;[1 1 1] Destroy Self when Player Passes
  (Utilities|Time|SetTimerbyEvent (delegate Custom|DestroySelf) 8.0))

(event Collision|EventActorBeginOverlap
  (params (OtherActor :type Actor%20Object%20Reference)))

(event EventTick
  (params (DeltaSeconds :type Float%20%28single-precision%29)))

(fn ConstructionScript)