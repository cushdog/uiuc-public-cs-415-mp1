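; BP_Healthpack is a timed health pickup that heals the player on contact.
; A timer set at BeginPlay destroys it after a few seconds if it is not collected.
; When BP_Player overlaps its box, it adds one health if below the cap and refreshes the player's health HUD text.
; It then destroys itself, even when health is already full.
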(event OnComponentBeginOverlap(Box)
  (params (OverlappedComponent :type Primitive%20Component%20Object%20Reference) (OtherActor :type Actor%20Object%20Reference) (OtherComp :type Primitive%20Component%20Object%20Reference) (OtherBodyIndex :type Integer) (bFromSweep :type Boolean) (SweepResult :type Hit%20Result%20Structure%20%28by%20ref%29))
  (bind _asbp_player (Utilities|Casting|CastToBP_Player OtherActor))
  ;[1 1 1] Increment Player Health
  (if (< (Variables|/Game/InfiniteMatrix/Blueprints/BP_Player.BP_Player_C|GetHealth _asbp_player) 4.0)
    (bind _result (Math|Float|IncrementFloat (Variables|/Game/InfiniteMatrix/Blueprints/BP_Player.BP_Player_C|GetHealth _asbp_player))
      (:%20%20
        (Variables|/Game/InfiniteMatrix/Blueprints/BP_Player.BP_Player_C|SetHealth _asbp_player _result)
        (Default|UpdateHealthText (Variables|/Game/InfiniteMatrix/Blueprints/BP_Player.BP_Player_C|GetHealthHUD _asbp_player)))))
  (Actor|DestroyActor))

(event Custom|DestroySelf
  ;[1 1 1] Destroy After a Certain Amount of Time
  (Actor|DestroyActor))

(event EventBeginPlay
  ;[1 1 1] Destroy After a Certain Amount of Time
  (Utilities|Time|SetTimerbyEvent (delegate Custom|DestroySelf) 8.0))

(event Collision|EventActorBeginOverlap
  (params (OtherActor :type Actor%20Object%20Reference)))

(event EventTick
  (params (DeltaSeconds :type Float%20%28single-precision%29)))

(fn ConstructionScript)